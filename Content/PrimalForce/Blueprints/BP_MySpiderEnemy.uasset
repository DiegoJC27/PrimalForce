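; Pooled spider enemy that damages other actors carrying a health component through a toggleable attack collider, ignoring fellow spiders.
; Losing health cancels the attack montage and pauses AI logic for a second.
; Death stops the AI, notifies the spawner and animation Blueprint, then tweens dither and fresnel material masks to fade out.
; When the dither fade completes, the spawner despawns it, and spawning restores full health.
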(event OnDeath(BP_HealthComponent)
  (bind _bp_runtimematerial (Variables|Default|GetBP_RuntimeMaterial))
  (bind _dithermask (Variables|Default|GetditherMask))
  (bind _fresnelmask (Variables|Default|GetFresnelMask))
  (bind _runtimematerial (Variables|/Game/PrimalForce/Blueprints/BP_RuntimeMaterial.BP_RuntimeMaterial_C|GetruntimeMaterial _bp_runtimematerial))
  (if (Variables|Default|GetisAlive)
    (Variables|Default|SetisAlive false)
    (CallFunction|DeactivateAttackCollider)
    (AI|Logic|StopLogic (Variables|/Script/AIModule.AIController|GetBrainComponent (AI|GetAIController self)) "")
    (Class|SpiderSpawneer|DisableSpiderIA (Variables|Default|GetSpawneerRef) self)
    (bind _asabp_spider (Utilities|Casting|CastToABP_Spider (Components|SkeletalMesh|GetAnimInstance (Variables|Character|GetMesh))))
    (Variables|/Game/Fab/Spider_animated_character/ABP_Spider.ABP_Spider_C|SetisAlive _asabp_spider false)
    (Utilities|FlowControl|Delay 1.0)
    (bind _returnvalue (Rendering|Material|GetScalarParameterValue _runtimematerial _dithermask :!class /Script/Engine.MaterialInstanceDynamic))
    (bind _value (|TweenFloat _returnvalue 0.0 2.0 "Linear")
      (:then
        (Rendering|Material|GetScalarParameterValue _runtimematerial _fresnelmask :!class /Script/Engine.MaterialInstanceDynamic)
        (bind _value_2 (|TweenFloat 0.0 0.0 2.0 "Linear" 0.0 0.0 1.0)
          (:then
            (Development|PrintText "Killed Spider"))
          (:ApplyEasing
            (Rendering|Material|SetScalarParameterValue _runtimematerial _fresnelmask _value_2 :!class /Script/Engine.MaterialInstanceDynamic)
            (Default|ApplyRuntimeMaterial _bp_runtimematerial (Utilities|Array|MakeArray (Variables|Character|GetMesh))))))
      (:ApplyEasing
        (Rendering|Material|SetScalarParameterValue _runtimematerial _dithermask _value :!class /Script/Engine.MaterialInstanceDynamic)
        (Default|ApplyRuntimeMaterial _bp_runtimematerial (Utilities|Array|MakeArray (Variables|Character|GetMesh))))
      (:OnComplete
        ;[0.15 0.15 0.15 0.5] Despawn
        (Class|SpiderSpawneer|DeSpawnSpider (Variables|Default|GetSpawneerRef) self)))))

(event OnComponentBeginOverlap(AttackCollision)
  (params (OverlappedComponent :type Primitive%20Component%20Object%20Reference) (OtherActor :type Actor%20Object%20Reference) (OtherComp :type Primitive%20Component%20Object%20Reference) (OtherBodyIndex :type Integer) (bFromSweep :type Boolean) (SweepResult :type Hit%20Result%20Structure%20%28by%20ref%29))
  (bind _returnvalue (Actor|GetComponentbyClass OtherActor "/Game/PrimalForce/Blueprints/BP_HealthComp.BP_HealthComp_C"))
  (if (not (Class|GameplayStatics|ObjectIsA OtherActor "BP_MySpiderEnemy_C"))
    (Utilities|IsValid _returnvalue
      (:Is%20Valid
        (Class|HealthComp|UpdateHealth _returnvalue (- 0.0 (Variables|Default|Getdamage)))))))

(event OnLoseHealth(BP_HealthComponent)
  (bind _asbp_spider_ai (Utilities|Casting|CastToBP_SpiderAI (Pawn|GetController)))
  (AI|Navigation|StopMovement _asbp_spider_ai)
  (AI|Logic|StopLogic (Variables|/Script/AIModule.AIController|GetBrainComponent _asbp_spider_ai) "")
  (Animation|StopAnimMontage "/Game/Fab/Spider_animated_character/spider_animated_character/SkeletalMeshes/AM_SpiderAttack.AM_SpiderAttack")
  (Class|SpiderEnemy|RecieveDamage)
  (Utilities|FlowControl|Delay 1.0)
  (Class|BrainComponent|RestartLogic (Variables|/Script/AIModule.AIController|GetBrainComponent _asbp_spider_ai)))

(event Custom|ActivateAttackCollider
  (Collision|SetCollisionEnabled (Variables|Default|GetAttackCollision) "QueryOnly"))

(event Custom|DeactivateAttackCollider
  (Collision|SetCollisionEnabled (Variables|Default|GetAttackCollision) "NoCollision"))

(event EventBeginPlay
  (CallFunction|DeactivateAttackCollider)
  (bind _outactors (Actor|GetAllActorsOfClass "/Game/PrimalForce/Blueprints/BP_SpiderSpawneer.BP_SpiderSpawneer_C"))
  (for _array_element _outactors
    (Variables|Default|SetSpawneerRef _array_element)))

(event EventOnDeSpawn
  (params (instigator :type Actor%20Object%20Reference))
  (CallFunction|DeactivateAttackCollider))

(event EventOnSpawn
  (params (instigator :type Actor%20Object%20Reference))
  (bind _bp_healthcomponent (Variables|Default|GetBP_HealthComponent))
  (Variables|/Game/PrimalForce/Blueprints/BP_HealthComp.BP_HealthComp_C|SetcurHp _bp_healthcomponent (Variables|/Game/PrimalForce/Blueprints/BP_HealthComp.BP_HealthComp_C|GetmaxHp _bp_healthcomponent))
  (CallFunction|DeactivateAttackCollider))

(event EventLifeTime
  (params (time :type Float%20%28single-precision%29)))

(fn ConstructionScript
  (bind _bp_healthcomponent (Variables|Default|GetBP_HealthComponent))
  (bind _output_get (Variables|/Game/PrimalForce/Blueprints/BP_HealthComp.BP_HealthComp_C|SetmaxHp _bp_healthcomponent (Variables|Default|GetmaxHealth)))
  (Variables|/Game/PrimalForce/Blueprints/BP_HealthComp.BP_HealthComp_C|SetcurHp _bp_healthcomponent _output_get))