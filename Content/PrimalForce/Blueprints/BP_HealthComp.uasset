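; BP_HealthComp is a health component that tracks an owner's hit points and reports changes to listeners.
; On BeginPlay it defaults a non-positive MaxHp to 100 and fills CurHp to it.
; UpdateHealth adds a signed delta, then fires a gain or lose dispatcher, or the death dispatcher once health reaches zero or below.
; CurHp is never clamped to MaxHp.
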(event EventBeginPlay
  (if (> (Variables|Default|GetmaxHp) 0.0)
    _
    (else
      (Variables|Default|SetmaxHp 1e+02)))
  (Variables|Default|SetcurHp (Variables|Default|GetmaxHp)))

(event EventUpdateHealth
  (params (plusLife :type Float%20%28single-precision%29))
  (bind _output_get (Variables|Default|SetcurHp (+ plusLife (Variables|Default|GetcurHp))))
  (if (> _output_get 0.0)
    (if (> plusLife 0.0)
      (Default|CallOnGainHealth)
      (else
        (Default|CallOnLoseHealth)))
    (else
      (Default|CallOnDeath))))