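; BP_RockProyectile is a rock projectile that deals fixed damage to spider enemies.
; OnSpawn re-enables its ProjectileMovement and launches it along the instigator's forward vector at ProyectileSpeed.
; Overlaps damage BP_MySpiderEnemy through its health component and hide the rock on anything except the player character.
; LifeTime hides it after a delay, so the actor is never destroyed here, which suggests reuse.
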(event OnComponentBeginOverlap(rootComp)
  (params (OverlappedComponent :type Primitive%20Component%20Object%20Reference) (OtherActor :type Actor%20Object%20Reference) (OtherComp :type Primitive%20Component%20Object%20Reference) (OtherBodyIndex :type Integer) (bFromSweep :type Boolean) (SweepResult :type Hit%20Result%20Structure%20%28by%20ref%29))
  (bind _asbp_my_spider_enemy (Utilities|Casting|CastToBP_MySpiderEnemy OtherActor)
    (:then
      (Default|UpdateHealth (Variables|/Game/PrimalForce/Blueprints/BP_MySpiderEnemy.BP_MySpiderEnemy_C|GetBP_HealthComponent _asbp_my_spider_enemy) -1e+02))
    (:CastFailed
      (Utilities|Casting|CastToBP_PlayerCharacter OtherActor
        (:CastFailed
          _))))
  (Class|ActorUtilities|ToggleActorHidden self true))

(event EventBeginPlay)

(event Collision|EventActorBeginOverlap
  (params (OtherActor :type Actor%20Object%20Reference)))

(event EventTick
  (params (DeltaSeconds :type Float%20%28single-precision%29)))

(event EventOnSpawn
  (params (instigator :type Actor%20Object%20Reference))
  (bind _projectilemovement (Variables|Default|GetProjectileMovement))
  (Components|Movement|SetUpdatedComponent (Variables|Default|GetProjectileMovement) (Variables|Transformation|GetRootComponent))
  (Variables|/Script/Engine.ProjectileMovementComponent|SetbSimulationEnabled _projectilemovement true)
  (Variables|/Script/Engine.MovementComponent|SetVelocity _projectilemovement (* (Transformation|GetActorForwardVector instigator) (Variables|Default|GetProyectileSpeed))))

(event EventLifeTime
  (params (time :type Float%20%28single-precision%29))
  (Utilities|FlowControl|Delay time)
  (Class|ActorUtilities|ToggleActorHidden self true))

(fn ConstructionScript)