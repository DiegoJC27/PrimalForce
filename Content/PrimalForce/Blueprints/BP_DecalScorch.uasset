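; BP_DecalScorch is a scorch mark decal Blueprint with a timed fade-out.
; BeginPlay creates and stores a dynamic material instance from the decal.
; The LifeTime event resets the material's lifetime opacity to full, then starts the decal's built-in fade after the given time.
; The fade leaves the owner alive, and nothing follows the closing delay that spans the wait and fade.
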(event Custom|ForceOpacity
  (Rendering|Material|SetScalarParameterValue (Variables|Default|GetRuntime%20mat) "Decal Lifetime Opacity" 1.0 :!class /Script/Engine.MaterialInstanceDynamic))

(event EventBeginPlay
  (bind _returnvalue (Rendering|Material|CreateDynamicMaterialInstance (Variables|Decal|GetDecal) :!class /Script/Engine.DecalComponent))
  (Variables|Default|SetRuntime%20mat _returnvalue))

(event EventLifeTime
  (params (time :type Float%20%28single-precision%29))
  (bind _fadeduration (Variables|Default|GetFadeDuration))
  (bind _decal (Variables|Decal|GetDecal)
    (:then
      (CallFunction|ForceOpacity)
      (Rendering|Components|Decal|SetFadeOut _decal time _fadeduration false)
      (Utilities|FlowControl|Delay (+ time _fadeduration)))
    (:else)))

(fn ConstructionScript)