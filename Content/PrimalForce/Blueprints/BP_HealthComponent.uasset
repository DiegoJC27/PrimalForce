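; BP_HealthComponent is a health component that tracks current and maximum HP for its owner.
; On BeginPlay it defaults a non-positive MaxHp to 100 and fills current HP to that maximum.
; UpdateHealth adds a signed value without clamping, then fires the OnGainHealth, OnLoseHealth or OnDeath dispatcher.
; Death fires on every update that leaves HP at or below zero, and a zero change counts as a loss.
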(event Custom|UpdateHealth
  (params (value :type Float%20%28double-precision%29))
  (bind _output_get (Variables|Default|SetcurHp (+ value (Variables|Default|GetcurHp))))
  (if (> _output_get 0.0)
    (if (> value 0.0)
      (Default|CallOnGainHealth)
      (else
        (Default|CallOnLoseHealth)))
    (else
      (Default|CallOnDeath))))

(event EventBeginPlay
  (if (> (Variables|Default|GetmaxHp) 0.0)
    _
    (else
      (Variables|Default|SetmaxHp 1e+02)))
  (Variables|Default|SetcurHp (Variables|Default|GetmaxHp)))