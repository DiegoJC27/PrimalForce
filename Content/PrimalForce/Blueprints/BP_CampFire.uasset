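; BP_CampFire is a campfire actor that cooks an egg delivered by the player and has its own health and lifebar.
; When a player carrying an egg hits its collider, it takes the egg, shows it on the fire and tells the game mode to start spawning spiders.
; Tick advances a progress bar widget while cooking.
; A FinishedCooking event stops the spawning, though nothing here calls it.
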(event OnComponentHit(Collider)
  (params (HitComponent :type Primitive%20Component%20Object%20Reference) (OtherActor :type Actor%20Object%20Reference) (OtherComp :type Primitive%20Component%20Object%20Reference) (NormalImpulse :type Vector :default "0, 0, 0") (Hit :type Hit%20Result%20Structure%20%28by%20ref%29))
  (bind _asbp_player_character (Utilities|Casting|CastToBP_PlayerCharacter OtherActor))
  (if (Variables|/Script/PrimalForce.PrimalForceCharacter|GethasEgg _asbp_player_character)
    (Default|ShowEgg _asbp_player_character false)
    (Variables|/Script/PrimalForce.PrimalForceCharacter|SethasEgg _asbp_player_character false)
    (CallFunction|StartCooking)))

(event OnLoseHealth(BP_HealthComp)
  (bind _bp_healthcomp (Variables|Default|GetBP_HealthComp))
  (bind _aswbp_tower_lifebar (Utilities|Casting|CastToWBP_TowerLifebar (UserInterface|GetWidget (Variables|Default|GetLifebar))))
  (Default|SetPercent _aswbp_tower_lifebar (/ (Variables|/Game/PrimalForce/Blueprints/BP_HealthComp.BP_HealthComp_C|GetcurHp _bp_healthcomp) (Variables|/Game/PrimalForce/Blueprints/BP_HealthComp.BP_HealthComp_C|GetmaxHp _bp_healthcomp))))

(event Custom|StartCooking
  (Rendering|SetVisibility (Variables|Default|GetEgg) true false)
  (bind _asbp_primal_force_game_mode (Utilities|Casting|CastToBP_PrimalForceGameMode (Game|GetGameMode)))
  (Default|StartSpawningSpiders _asbp_primal_force_game_mode)
  (Rendering|SetVisibility (Variables|Default|GetProgressBar) true false)
  (Variables|Default|SetcookingEgg true))

(event Custom|Finished%20Cooking
  (bind _asbp_primal_force_game_mode (Utilities|Casting|CastToBP_PrimalForceGameMode (Game|GetGameMode)))
  (Default|StopSpawningSpiders _asbp_primal_force_game_mode))

(event EventBeginPlay
  (Rendering|SetVisibility (Variables|Default|GetProgressBar) false false))

(event EventTick
  (params (DeltaSeconds :type Float%20%28single-precision%29))
  (if (Variables|Default|GetcookingEgg)
    (bind _output_get (Variables|Default|SetcurTime (+ (Variables|Default|GetcurTime) DeltaSeconds)))
    (bind _aswbp_progress_bar_fogata (Utilities|Casting|CastToWBP_ProgressBarFogata (UserInterface|GetWidget (Variables|Default|GetProgressBar))))
    (Default|SetProgressPercent _aswbp_progress_bar_fogata (/ _output_get (Variables|Default|GettimeToCook)))))

(fn ConstructionScript)