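; BP_SpiderDefender is a spider enemy that turns to face the player each tick and plays an attack montage when in range.
; Its toggleable attack collider damages overlapped actors with a health component, excluding other spider defenders.
; Losing health interrupts the attack with a damage montage.
; Death updates the spider AnimBP, disables the collider, then tweens dither and fresnel material parameters to fade the mesh before destroying the actor.
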(event OnDeath(BP_HealthComponent)
  (bind _bp_runtimematerial (Variables|Default|GetBP_RuntimeMaterial))
  (bind _dithermask (Variables|Default|GetditherMask))
  (bind _fresnelmask (Variables|Default|GetFresnelMask))
  (bind _runtimematerial (Variables|/Game/PrimalForce/Blueprints/BP_RuntimeMaterial.BP_RuntimeMaterial_C|GetruntimeMaterial _bp_runtimematerial))
  (if (Variables|Default|GetisAlive)
    (Variables|Default|SetisAlive false)
    (CallFunction|DeactivateAttackCollider)
    (bind _asabp_spider (Utilities|Casting|CastToABP_Spider (Components|SkeletalMesh|GetAnimInstance (Variables|Character|GetMesh))))
    (Variables|/Game/Fab/Spider_animated_character/ABP_Spider.ABP_Spider_C|SetisAlive _asabp_spider false)
    (Utilities|FlowControl|Delay 1.0)
    (bind _returnvalue (Rendering|Material|GetScalarParameterValue _runtimematerial _dithermask :!class /Script/Engine.MaterialInstanceDynamic))
    (bind _value (|TweenFloat _returnvalue 0.0 2.0 "Linear")
      (:then
        (Rendering|Material|GetScalarParameterValue _runtimematerial _fresnelmask :!class /Script/Engine.MaterialInstanceDynamic)
        (bind _value_2 (|TweenFloat 0.0 0.0 2.0 "Linear" 0.0 0.0 1.0)
          (:then
            (Development|PrintText "Killed Spider"))
          (:ApplyEasing
            (Rendering|Material|SetScalarParameterValue _runtimematerial _fresnelmask _value_2 :!class /Script/Engine.MaterialInstanceDynamic)
            (Default|ApplyRuntimeMaterial _bp_runtimematerial (Utilities|Array|MakeArray (Variables|Character|GetMesh))))))
      (:ApplyEasing
        (Rendering|Material|SetScalarParameterValue _runtimematerial _dithermask _value :!class /Script/Engine.MaterialInstanceDynamic)
        (Default|ApplyRuntimeMaterial _bp_runtimematerial (Utilities|Array|MakeArray (Variables|Character|GetMesh))))
      (:OnComplete
        (Actor|DestroyActor)))))

(event OnLoseHealth(BP_HealthComponent)
  (Animation|StopAnimMontage "/Game/Caveman/Blueprints/AM_DamageAraña.AM_DamageAraña")
  (Animation|StopAnimMontage "/Game/Fab/Spider_animated_character/spider_animated_character/SkeletalMeshes/AM_SpiderAttack.AM_SpiderAttack")
  (Animation|Montage|PlayMontage (Variables|Character|GetMesh) "/Game/Caveman/Blueprints/AM_DamageAraña.AM_DamageAraña"
    (:then
      (Utilities|FlowControl|Delay 1.0))))

(event OnComponentBeginOverlap(AttackCollision)
  (params (OverlappedComponent :type Primitive%20Component%20Object%20Reference) (OtherActor :type Actor%20Object%20Reference) (OtherComp :type Primitive%20Component%20Object%20Reference) (OtherBodyIndex :type Integer) (bFromSweep :type Boolean) (SweepResult :type Hit%20Result%20Structure%20%28by%20ref%29))
  (bind _returnvalue (Actor|GetComponentbyClass OtherActor "/Game/PrimalForce/Blueprints/BP_HealthComp.BP_HealthComp_C"))
  (if (not (Class|GameplayStatics|ObjectIsA OtherActor "BP_SpiderDefender_C"))
    (Utilities|IsValid _returnvalue
      (:Is%20Valid
        (Class|HealthComp|UpdateHealth _returnvalue (- 0.0 (Variables|Default|Getdamage)))))))

(event Custom|LookAtPlayer
  (Transformation|SetActorRotation (Math|Rotator|FindLookatRotation (Transformation|GetActorLocation self) (Transformation|GetActorLocation (Variables|Default|GetplayerRef)))))

(event Custom|DeactivateAttackCollider
  (Collision|SetCollisionEnabled (Variables|Default|GetAttackCollision) "NoCollision"))

(event Custom|ActivateAttackCollider
  (Collision|SetCollisionEnabled (Variables|Default|GetAttackCollision) "QueryOnly"))

(event Custom|Attack
  (if (not (Variables|Default|GetisAttacking))
    (if (<= (Transformation|GetDistanceTo self (Variables|Default|GetplayerRef)) (Variables|Default|GetattackRange))
      (Variables|Default|SetisAttacking true)
      (Animation|Montage|PlayMontage (Variables|Character|GetMesh) "/Game/Fab/Spider_animated_character/spider_animated_character/SkeletalMeshes/AM_SpiderAttack.AM_SpiderAttack"
        (:then
          (Utilities|FlowControl|Delay 1.0)
          (Variables|Default|SetisAttacking false))))))

(event EventBeginPlay
  (bind _bp_healthcomponent (Variables|Default|GetBP_HealthComponent))
  (Variables|/Game/PrimalForce/Blueprints/BP_HealthComp.BP_HealthComp_C|SetcurHp _bp_healthcomponent (Variables|/Game/PrimalForce/Blueprints/BP_HealthComp.BP_HealthComp_C|GetmaxHp _bp_healthcomponent))
  (CallFunction|DeactivateAttackCollider)
  (bind _asprimal_force_character (Utilities|Casting|CastToPrimalForceCharacter (Game|GetPlayerCharacter 0)))
  (Variables|Default|SetplayerRef _asprimal_force_character))

(event EventTick
  (params (DeltaSeconds :type Float%20%28single-precision%29))
  (CallFunction|LookatPlayer)
  (CallFunction|Attack))

(fn ConstructionScript)